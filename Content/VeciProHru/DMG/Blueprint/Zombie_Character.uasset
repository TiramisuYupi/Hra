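; Zombie enemy character that wanders between random tagged actors, chases the first-person player and displays its health.
; A patrol loop restarts two seconds after each successful move; AI Perception updates redirect it to the player, and forgetting the player resumes patrol.
; Sphere hits apply damage only to other Zombie_Character actors.
; Incoming damage is scaled up a hundredfold, subtracted from health and sent to the health widget, with no death handling.
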(event `self.Sphere.OnComponentHit`
  (params (HitComponent :type "PrimitiveComponent Object Reference") (OtherActor :type "Actor Object Reference") (OtherComp :type "PrimitiveComponent Object Reference") (NormalImpulse :type "Vector Structure") (Hit :type "HitResult Structure (by ref)"))
  (bind _aszombie_character (cast `/Game/VeciProHru/DMG/Blueprint/Zombie_Character` OtherActor))
  (`GameplayStatics.ApplyDamage` _aszombie_character 20.0))

(event `self.ReceiveAnyDamage`
  (params (Damage :type "Float (single-precision)") (DamageType :type "DamageType Object Reference") (InstigatedBy :type "Controller Object Reference") (DamageCauser :type "Actor Object Reference"))
  (bind _output_get (set `self.CurrectHealth` (`KismetMathLibrary.FTrunc` (- (`self.CurrectHealth`) (* Damage 100.0)))))
  (`/Game/VeciProHru/DMG/UI/WBP_EnemyHealth.Update Health` (`self.WBP Enemy Health`) _output_get))

(event `self.ReceiveBeginPlay`
  (`|ExecutionSequence`
    (:`then_0`
      (bind _aswbp_enemy_health (cast `/Game/VeciProHru/DMG/UI/WBP_EnemyHealth` (`WidgetComponent.GetUserWidgetObject` (`self.Widget`))))
      (bind _output_get (set `self.WBP Enemy Health` _aswbp_enemy_health))
      (set `/Game/VeciProHru/DMG/UI/WBP_EnemyHealth.CurrentHealth` (`self.CurrectHealth`) _output_get)
      (set `/Game/VeciProHru/DMG/UI/WBP_EnemyHealth.MaxHealth` (`self.MaxHealth`) _output_get))
    (:`then_1`
      (add `AIPerceptionComponent.OnTargetPerceptionForgotten` (`self.AIPerception`) (delegate `OnTargetPerceptionForgotten_Event`))
      (bind _outactors (`GameplayStatics.GetAllActorsWithTag` (`self.Tag`) :!label _label))
      (`|AIMoveTo` self (0.0 0.0 0.0) (`KismetArrayLibrary.Array_Random` _outactors)
        (:`OnSuccess`
          (`KismetSystemLibrary.Delay` 2.0)
          (goto _label))))))

(event `OnTargetPerceptionForgotten_Event`
  (params (Actor :type "Actor Object Reference")))

(event `self.AIPerception.OnTargetPerceptionForgotten`
  (params (Actor :type "Actor Object Reference"))
  (cast `/Game/FirstPerson/Blueprints/BP_FirstPersonCharacter` Actor)
  (set `CharacterMovementComponent.MaxWalkSpeed` 100.0 (`self.CharacterMovement`))
  (goto _label))

(event `self.AIPerception.OnTargetPerceptionUpdated`
  (params (Actor :type "Actor Object Reference") (Stimulus :type "AIStimulus Structure"))
  (bind _asbp_first_person_character (cast `/Game/FirstPerson/Blueprints/BP_FirstPersonCharacter` Actor))
  (set `CharacterMovementComponent.MaxWalkSpeed` 100.0 (`self.CharacterMovement`))
  (`|AIMoveTo` self (0.0 0.0 0.0) _asbp_first_person_character))

(fn `UserConstructionScript`)