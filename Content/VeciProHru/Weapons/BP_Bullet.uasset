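; Bullet actor that damages Squidle and Zombie characters on contact.
; Its static mesh's begin-overlap event applies fixed damage and destroys the bullet, counting Squidle hits only on the character's Mesh component, but Zombie hits on any component.
; Other overlaps leave the bullet alive, and an unconnected tag-based damage branch never runs.
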(event `self.StaticMesh.OnComponentBeginOverlap`
  (params (OverlappedComponent :type "PrimitiveComponent Object Reference") (OtherActor :type "Actor Object Reference") (OtherComp :type "PrimitiveComponent Object Reference") (OtherBodyIndex :type Integer) (bFromSweep :type Boolean) (SweepResult :type "HitResult Structure (by ref)"))
  (bind _assquidle_character (cast `/Game/VeciProHru/Squidle/Squidle_Character` OtherActor)
    (:`then`
      (if (== OtherComp (`Character.Mesh` _assquidle_character))
        (`GameplayStatics.ApplyDamage` _assquidle_character 20.0)
        (`self.K2_DestroyActor` :!label _label)))
    (:`CastFailed`
      (bind _aszombie_character (cast `/Game/VeciProHru/DMG/Blueprint/Zombie_Character` OtherActor))
      (`GameplayStatics.ApplyDamage` _aszombie_character 20.0)
      (goto _label))))

(fn `UserConstructionScript`)